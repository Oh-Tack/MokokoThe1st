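; Player attack component that runs a three-hit melee combo on left mouse input.
; It caches the owning player character's mesh, then plays the montage matching the combo counter when not attacking and allowed to attack.
; Each montage's notify reopens input and advances or wraps the counter.
; A one-second timer, set as each montage starts, resets the combo; blocked input prints the attack flags.
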(event `self.ReceiveBeginPlay`
  (bind _asbp_player_charater (cast `/Game/Blueprints/Player/BP_PlayerCharater` (`self.GetOwner`)))
  (bind _output_get (set `self.As BP Player Charater` _asbp_player_charater))
  (set `self.PlayerMesh` (`Character.Mesh` _output_get)))

(event `EnhancedInput|/Game/Inputs/Actions/IA_Mouse_Left`
  (params (ActionValue :type Boolean) (ElapsedSeconds :type "Float (double-precision)") (TriggeredSeconds :type "Float (double-precision)") (InputAction :type "InputAction Object Reference" :default "/Game/Inputs/Actions/IA_Mouse_Left.IA_Mouse_Left"))
  (bind _playermesh (`self.PlayerMesh`))
  (:`Started`
    (if (and (not (`self.bIsAttacking`)) (`self.bCanAttack`))
      (set `self.bIsAttacking` true)
      (switch `int` (`self.ComboCounter`)
        (:`0`
          (`|PlayMontage` _playermesh "/Game/Characters/Player/Animations/Attack/Player_ComboAttack1_Montage.Player_ComboAttack1_Montage"
            (:`then`
              (`KismetSystemLibrary.K2_SetTimerDelegate` (delegate `ResetCounter`) 1.0 :!label _label))
            (:`OnNotifyBegin`
              (set `self.bIsAttacking` false)
              (set `self.ComboCounter` 1))))
        (:`1`
          (`|PlayMontage` _playermesh "/Game/Characters/Player/Animations/Attack/Player_ComboAttack2_Montage.Player_ComboAttack2_Montage" 0.5
            (:`then`
              (goto _label))
            (:`OnNotifyBegin`
              (set `self.bIsAttacking` false)
              (set `self.ComboCounter` 2))))
        (:`2`
          (`|PlayMontage` _playermesh "/Game/Characters/Player/Animations/Attack/Player_ComboAttack3_Montage.Player_ComboAttack3_Montage"
            (:`then`
              (goto _label))
            (:`OnNotifyBegin`
              (set `self.bIsAttacking` false)
              (set `self.ComboCounter` 0)))))
      (else
        (`KismetSystemLibrary.PrintString` (`KismetTextLibrary.Conv_TextToString` (`|FormatText` "{0} is attack | {1} can attack" (`self.bIsAttacking`) (`self.bCanAttack`))))))))

(event `ResetCounter`
  (set `self.ComboCounter` 0))