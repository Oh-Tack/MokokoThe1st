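; Player controller for top-down, click-to-move control, with a basic attack and a key that triggers enemy patterns.
; Right-click traces under the cursor: holding steers the pawn toward the hit, while a short press path-moves there with a Niagara cursor effect.
; Left-click plays the attack montage, gated by a player state enum to block repeat clicks.
; J calls ExecutePattern on every BP_Enemy; Enhanced Input mapping is added on BeginPlay.
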(event `EnhancedInput|/Game/Inputs/Actions/IA_J`
  (params (ActionValue :type "Float (double-precision)") (ElapsedSeconds :type "Float (double-precision)") (TriggeredSeconds :type "Float (double-precision)") (InputAction :type "InputAction Object Reference" :default "/Game/Inputs/Actions/IA_J.IA_J"))
  ; 플레이어 J 입력 받기
  (:`Started`
    (bind _outactors (`GameplayStatics.GetAllActorsOfClass` "/Game/Blueprints/Boss/BP_Enemy.BP_Enemy_C"))
    (for _array_element _outactors
      (`/Game/Blueprints/Boss/BP_Enemy.ExecutePattern` _array_element))))

(event `self.ReceiveBeginPlay`
  (bind _returnvalue (subsystem `EnhancedInputLocalPlayerSubsystem`))
  ; Enhanced Input 초기 설정
  (`/Engine/EditorBlueprintResources/StandardMacros.IsValid` _returnvalue
    (:`Is Valid`
      (`EnhancedInputSubsystemInterface.AddMappingContext` _returnvalue "/Game/Inputs/IMC_PlayerInput.IMC_PlayerInput" 0 (struct)))))

(event `EnhancedInput|/Game/Inputs/Actions/IA_Mouse_Right`
  (params (ActionValue :type Boolean) (ElapsedSeconds :type "Float (double-precision)") (TriggeredSeconds :type "Float (double-precision)") (InputAction :type "InputAction Object Reference" :default "/Game/Inputs/Actions/IA_Mouse_Right.IA_Mouse_Right"))
  (bind (_hit _loc) (`self.GetLocationUnderCursor`))
  (bind (_hit_2 _loc_2) (`self.GetLocationUnderCursor`))
  ; 오른쪽 마우스 클릭 - 이동
  (:`Triggered`
    (if _hit
      (bind _output_get (set `self.CachedDestination` _loc))
      (`self.Follow` _output_get)))
  (:`Started`
    (`self.StopMovement`)
    (if _hit_2
      (set `self.CachedDestination` _loc_2)))
  (:`Canceled`
    (if (< ElapsedSeconds (`self.PressedThreshold`)) :!label _label
      (`self.MoveTo` (`self.CachedDestination`))))
  (:`Completed`
    (goto _label)))

(event `EnhancedInput|/Game/Inputs/Actions/IA_Mouse_Left`
  (params (ActionValue :type Boolean) (ElapsedSeconds :type "Float (double-precision)") (TriggeredSeconds :type "Float (double-precision)") (InputAction :type "InputAction Object Reference" :default "/Game/Inputs/Actions/IA_Mouse_Left.IA_Mouse_Left"))
  ; 마우스 왼쪽 클릭 - 기본 공격 # 중복 클릭 수정
  (:`Started`
    (if (`|EnumEquality` (`self.EPlayerState`) "NewEnumerator0")
      (set `self.EPlayerState` "NewEnumerator2")
      (bind _asbp_player_charater (cast `/Game/Blueprints/Player/BP_PlayerCharater` (`GameplayStatics.GetPlayerCharacter` 0)))
      (`Character.PlayAnimMontage` _asbp_player_charater "/Game/Characters/Player/Animations/AM_Player_Attack.AM_Player_Attack" 1.0 "None"))))

(fn `Follow`
  (params (Loc :type "Vector Structure"))
  (bind _returnvalue (`self.K2_GetPawn`))
  (`Pawn.AddMovementInput` _returnvalue (`KismetMathLibrary.GetDirectionUnitVector` (`self.K2_GetActorLocation` _returnvalue) Loc) 1.0 false))

(fn `GetLocationUnderCursor`
  (returns (Hit :type Boolean) (Loc :type "Vector Structure"))
  (bind (_bblockinghit _binitialoverlap _time _distance _location) (`GameplayStatics.BreakHitResult` (`self.GetHitResultUnderCursorByChannel` "TraceTypeQuery1")))
  (return _bblockinghit _location))

(fn `MoveTo`
  (params (Loc :type "Vector Structure"))
  (`AIBlueprintHelperLibrary.SimpleMoveToLocation` self Loc)
  (`NiagaraFunctionLibrary.SpawnSystemAtLocation` (`self.FXCursor`) Loc))

(fn `UserConstructionScript`)