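; StateTree task that starts a boss enemy's attack pattern and requests transitions based on the boss counter state.
; On entry it calls ExecutePattern on the Enemy if it is valid and neither countering nor attacking.
; The latent tick requests a normal-priority transition when BossCounter is set.
; Parallel Enter and Tick graphs repeat this logic, except Tick requests a transition on both branches.
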(event `self.ReceiveLatentEnterState`
  (params (Transition :type "StateTreeTransitionResult Structure (by ref)"))
  (`/Engine/EditorBlueprintResources/StandardMacros.IsValid` (`self.Enemy`)
    (:`Is Valid`
      (if (and (== (`/Game/Blueprints/Boss/BP_Enemy.Boss_Counter` (`self.Enemy`)) false) (== (`/Game/Blueprints/Boss/BP_Enemy.bIsAttacking` (`self.Enemy`)) false))
        (`/Game/Blueprints/Boss/BP_Enemy.ExecutePattern` (`self.Enemy`))))))

(event `self.ReceiveLatentTick`
  (params (DeltaTime :type "Float (single-precision)"))
  (`/Engine/EditorBlueprintResources/StandardMacros.IsValid` (`self.Enemy`)
    (:`Is Valid`
      (if (== (`/Game/Blueprints/Boss/BP_Enemy.Boss_Counter` (`self.Enemy`)) true)
        (`self.RequestTransition` (struct))))))

(fn `Enter`
  (`/Engine/EditorBlueprintResources/StandardMacros.IsValid` (`self.Enemy`)
    (:`Is Valid`
      (if (and (== (`/Game/Blueprints/Boss/BP_Enemy.Boss_Counter` (`self.Enemy`)) false) (== (`/Game/Blueprints/Boss/BP_Enemy.bIsAttacking` (`self.Enemy`)) false))
        (`/Game/Blueprints/Boss/BP_Enemy.ExecutePattern` (`self.Enemy`))))))

(fn `Tick`
  (`/Engine/EditorBlueprintResources/StandardMacros.IsValid` (`self.Enemy`)
    (:`Is Valid`
      (if (== (`/Game/Blueprints/Boss/BP_Enemy.Boss_Counter` (`self.Enemy`)) true)
        (`self.RequestTransition` (struct))
        (else
          (`self.RequestTransition` (struct)))))))