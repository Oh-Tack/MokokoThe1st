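; Boss enemy with an attached sword, four attack patterns, a counter stance, HP-triggered clashes and death, coordinated through StateTree events.
; A delayed Tick loop checks HP, randomly picks the next action type without repeating the last roll, and signals attack start.
; Patterns use teleports, montages, a box-trace knockback strike and spawned hazards, mostly ending via timers.
; A specific player attack type during the counter window triggers a counter-hit event and disables sword collision.
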(event `self.ReceiveBeginPlay`
  ; 게임 시작 후 검 부착
  (bind _returnvalue (`|SpawnActorFromClass` "/Game/Blueprints/Boss/BP_SWORD.BP_SWORD_C" (`KismetMathLibrary.MakeTransform` (0.0 0.0 0.0)) "Undefined" "MultiplyWithRoot" null null))
  (bind _output_get (set `self.Sword` _returnvalue))
  (`self.K2_AttachToComponent` _output_get (`self.Mesh`) "Sword_Socket" "SnapToTarget" "SnapToTarget" "SnapToTarget" true)
  (bind _asbp_player_charater (cast `/Game/Characters/Player/Blueprints/BP_PlayerCharater` (`GameplayStatics.GetPlayerCharacter` 0)))
  (set `self.As BP Player Charater` _asbp_player_charater)
  (if (== (`self.Boss_CHP`) 0.0)
    (set `self.Boss_CHP` (`self.Boss_MHP`)))
  (bind _returnvalue_2 (`GameplayStatics.GetActorOfClass` "/Game/Characters/Boss/BossSpawnPoint.BossSpawnPoint_C"))
  (set `self.BossSpawnPoint` _returnvalue_2)
  (bind _returnvalue_3 (`GameplayStatics.GetActorOfClass` "/Game/Characters/Boss/ClashPoint.ClashPoint_C"))
  (set `self.Clash Point` _returnvalue_3))

(event `self.CapsuleComponent.OnComponentBeginOverlap`
  (params (OverlappedComponent :type "PrimitiveComponent Object Reference") (OtherActor :type "Actor Object Reference") (OtherComp :type "PrimitiveComponent Object Reference") (OtherBodyIndex :type Integer) (bFromSweep :type Boolean) (SweepResult :type "HitResult Structure (by ref)"))
  ; 카운터 피격 로직(그로기 완성 )
  (`KismetSystemLibrary.PrintString` (`KismetSystemLibrary.GetDisplayName` OtherComp)))

(event `RemovePatternEvent`
  ; 패턴 소환 후 삭제 로직
  (`StateTreeComponent.SendStateTreeEvent` (`self.StateTree`) (make `StateTreeEvent` (struct :`TagName` "Boss.PatternEnd"))))

(event `RemovePatternEvent2`
  ; 패턴 소환 후 삭제 로직
  (`StateTreeComponent.SendStateTreeEvent` (`self.StateTree`) (make `StateTreeEvent` (struct :`TagName` "Boss.PatternEnd"))))

(event `self.ReceiveAnyDamage`
  (params (Damage :type "Float (single-precision)") (DamageType :type "DamageType Object Reference") (InstigatedBy :type "Controller Object Reference") (DamageCauser :type "Actor Object Reference"))
  ; 카운터 피격 로직(그로기 완성 )
  (bind _asbp_player_attack_base (cast `/Game/Core/BP_Player_Attack_Base` DamageType))
  (set `self.As BP Player Attack Base` _asbp_player_attack_base)
  (`self.UpdateBossHP` Damage)
  (if (and (`self.Boss_Counter`) (`|EnumEquality` (`/Game/Core/BP_Player_Attack_Base.PlayerAttackType` (`self.As BP Player Attack Base`)) "NewEnumerator0"))
    (`StateTreeComponent.SendStateTreeEvent` (`self.StateTree`) (make `StateTreeEvent` (struct :`TagName` "Boss.HitCounter")))
    (`PrimitiveComponent.SetCollisionEnabled` (`/Game/Blueprints/Boss/BP_SWORD.AttackCollision` (`self.Sword`)) "NoCollision")))

(event `self.ReceiveTick`
  (params (DeltaSeconds :type "Float (single-precision)"))
  ; 패턴 반복
  (`KismetSystemLibrary.Delay` 5.0)
  (`self.CheckBossHP`)
  (`self.DecideNextPattern`)
  (`StateTreeComponent.SendStateTreeEvent` (`self.StateTree`) (make `StateTreeEvent` (struct :`TagName` "Boss.StartAttack")))
  ;; 타겟팅
  (if (`self.bIsTargeting`)
    (`self.BossPlayerTargeting`)))

(event `RemoveSword`
  ; 패턴 소환 후 삭제 로직
  (`self.K2_DestroyActor` (`self.SpawnSword`)))

(event `RemoveVFX`
  ; 패턴 1
  (`GameplayStatics.PlaySound2D` "/Game/Characters/Boss/dragon-studio-armor-impact-from-sword-393843.dragon-studio-armor-impact-from-sword-393843" 1.0 1.0 0.0 null null)
  (set `self.bIsTargeting` false)
  (`|SpawnActorFromClass` "/Game/Blueprints/Boss/BP_VFX.BP_VFX_C" (`KismetMathLibrary.MakeTransform` (`self.K2_GetActorLocation`) (`self.K2_GetActorRotation`)) "Undefined" "MultiplyWithRoot" null null)
  (`StateTreeComponent.SendStateTreeEvent` (`self.StateTree`) (make `StateTreeEvent` (struct :`TagName` "Boss.PatternEnd"))))

(event `Delay Parttern`
  (bind _returnvalue (+ (`SceneComponent.GetSocketLocation` (`self.Mesh`) "hand_Isocket") (* (`self.GetActorForwardVector`) 150.0)))
  ; 패턴 2
  (set `self.bIsTargeting` false)
  ;; 애니메이션
  (`self.PlayAnimMontage` "/Game/Characters/Boss/Animations/Boss_Spell_Cast_Anim1_Montage.Boss_Spell_Cast_Anim1_Montage")
  (`NiagaraFunctionLibrary.SpawnSystemAtLocation` "/Game/Effects/VFX_Niagara/NS_Dash_Vampire.NS_Dash_Vampire" _returnvalue (`self.K2_GetActorRotation`) (1.0 1.0 1.0) false)
  (bind _outhits (`KismetSystemLibrary.BoxTraceMultiForObjects` :`Start` (+ _returnvalue (0.0 0.0 50.0)) :`End` (+ (+ (* (`self.GetActorForwardVector`) 800.0) (`self.K2_GetActorLocation`)) (0.0 0.0 50.0)) :`HalfSize` (10.0 50.0 50.0) :`Orientation` (`self.K2_GetActorRotation`) :`ObjectTypes` (`|MakeArray` "ObjectTypeQuery3" :!type "EObjectTypeQuery Enum") :`DrawDebugType` "ForDuration"))
  (for _ _outhits
    (`GameplayStatics.ApplyDamage` (`self.As BP Player Charater`) 20.0 null null "/Game/Core/BP_DamageType_Hit.BP_DamageType_Hit_C")
    (`self.LaunchCharacter` (`self.As BP Player Charater`) (* (- (`self.K2_GetActorLocation` (`self.As BP Player Charater`)) _returnvalue) (`self.Power`)) true true) ; 넉백
    (`StateTreeComponent.SendStateTreeEvent` (`self.StateTree`) (make `StateTreeEvent` (struct :`TagName` "Boss.PatternEnd"))))
  (`StateTreeComponent.SendStateTreeEvent` (`self.StateTree`) (make `StateTreeEvent` (struct :`TagName` "Boss.PatternEnd"))))

(event `Crash`
  ; 격돌 생성
  (`self.ClashStart`)
  (`|SpawnActorFromClass` "/Game/Cinematic/BluePrint/BP_EnterClash.BP_EnterClash_C" (`KismetMathLibrary.MakeTransform` (`self.K2_GetActorLocation` (`self.Clash Point`))) "Undefined" "MultiplyWithRoot" null null)
  (`KismetSystemLibrary.Delay` 5.0)
  (`StateTreeComponent.SendStateTreeEvent` (`self.StateTree`) (make `StateTreeEvent` (struct :`TagName` "Boss.EndClash"))))

(event `Event_EnableHitBox`
  ; BP_Sword 어택 콜리전
  (`PrimitiveComponent.SetCollisionEnabled` (`/Game/Blueprints/Boss/BP_SWORD.AttackCollision` (`self.Sword`)) "QueryOnly"))

(event `Event_DisableHitBox`
  ; BP_Sword 어택 콜리전
  (`PrimitiveComponent.SetCollisionEnabled` (`/Game/Blueprints/Boss/BP_SWORD.AttackCollision` (`self.Sword`)) "NoCollision"))

(fn `BossCrash`
  (`self.K2_SetActorLocation` (`self.K2_GetActorLocation` (`self.BossSpawnPoint`)))
  (`KismetSystemLibrary.K2_SetTimerDelegate` (`|CreateDelegate` :!event `Crash`) 2.0))

(fn `BossPlayerTargeting`
  (bind (_returnvalue_roll _returnvalue_pitch _returnvalue_yaw) (`KismetMathLibrary.BreakRotator` (`KismetMathLibrary.Conv_VectorToRotator` (- (`self.K2_GetActorLocation` (`GameplayStatics.GetPlayerCharacter` 0)) (`self.K2_GetActorLocation`)))))
  (`self.K2_SetActorRotation` (`KismetMathLibrary.MakeRotator` 0.0 0.0 _returnvalue_yaw)))

(fn `CheckBossHP`
  (`|ExecutionSequence`
    (:`then_0`
      (if (== (`self.Boss_CHP`) 0.0)
        (`StateTreeComponent.SendStateTreeEvent` (`self.StateTree`) (make `StateTreeEvent` (struct :`TagName` "Boss.Dead")))))
    (:`then_1`
      (if (and (<= (* (/ (`self.Boss_CHP`) (`self.Boss_MHP`)) (`self.TotalLine`)) 50.0) (not (`self.bIsClashTriggered`)))
        (set `self.bIsClashTriggered` true)
        (`StateTreeComponent.SendStateTreeEvent` (`self.StateTree`) (make `StateTreeEvent` (struct :`TagName` "Boss.StartClash")))))
    (:`then_2`
      (if (and (<= (* (/ (`self.Boss_CHP`) (`self.Boss_MHP`)) (`self.TotalLine`)) 75.0) (not (`self.bIsClashTrigger75`)))
        (set `self.bIsClashTrigger75` true)
        (`StateTreeComponent.SendStateTreeEvent` (`self.StateTree`) (make `StateTreeEvent` (struct :`TagName` "Boss.StartClash")))))))

(fn `DecideNextPattern`
  (while (== (`self.RN1`) (`self.CP1`))
    (set `self.RN1` (`KismetMathLibrary.RandomIntegerInRange` 1 5)))
  (bind _output_get (set `self.CP1` (`self.RN1`)))
  (switch `int` _output_get
    (:`1`
      (set `self.NextActionType` 0 :!label _label))
    (:`2`
      (goto _label))
    (:`3`
      (goto _label))
    (:`4`
      (goto _label))
    (:`5`
      (set `self.NextActionType` 1))))

(fn `ExecutePattern`
  ; 무작위 패턴 사용(중복 제외)
  ;; 중복 제외 로직
  (while (== (`self.RandomNum`) (`self.CurrentPattern`))
    (set `self.RandomNum` (`KismetMathLibrary.RandomIntegerInRange` 1 4)))
  (bind _output_get (set `self.CurrentPattern` (`self.RandomNum`)))
  (switch `int` _output_get
    (:`1`
      (`self.Pattern_Attack_01`))
    (:`2`
      (`self.Pattern_Attack_02`))
    (:`3`
      (`self.Pattern_Attack_03`))
    (:`4`
      (`self.Pattern_Attack_04`))))

(fn `Pattern_Attack_01`
  (bind _returnvalue (`GameplayStatics.GetPlayerCharacter` 0))
  ; Commen플레이어 위치 + a 텔레포트
  (`StateTreeComponent.SendStateTreeEvent` (`self.StateTree`) (make `StateTreeEvent` (struct :`TagName` "Boss.StartPattern")))
  (`self.K2_SetActorLocation` (+ (`self.K2_GetActorLocation` _returnvalue) (* (`self.GetActorForwardVector` _returnvalue) -200.0)) false true)
  (`self.BossPlayerTargeting`)
  (bind _returnvalue_2 (`self.PlayAnimMontage` "/Game/Characters/Boss/Animations/Boss_act1.Boss_act1"))
  (`KismetSystemLibrary.K2_SetTimerDelegate` (`|CreateDelegate` :!event `RemoveVFX`) _returnvalue_2))

(fn `Pattern_Attack_02`
  (bind _returnvalue (`GameplayStatics.GetPlayerCharacter` 0))
  (`StateTreeComponent.SendStateTreeEvent` (`self.StateTree`) (make `StateTreeEvent` (struct :`TagName` "Boss.StartPattern")))
  ; 백스텝
  (`self.K2_SetActorLocation` (+ (`self.K2_GetActorLocation` _returnvalue) (* (`self.GetActorForwardVector` _returnvalue) -300.0)))
  (`self.BossPlayerTargeting`)
  (`self.LaunchCharacter` (* (* (`self.GetActorForwardVector`) -1.0) 1000.0))
  (`KismetSystemLibrary.K2_SetTimerDelegate` (`|CreateDelegate` :!event `Delay Parttern`) 1.0))

(fn `Pattern_Attack_03`
  ; 패턴 Spawn
  (`self.BossPlayerTargeting`)
  (`StateTreeComponent.SendStateTreeEvent` (`self.StateTree`) (make `StateTreeEvent` (struct :`TagName` "Boss.StartPattern")))
  (bind _returnvalue (`|SpawnActorFromClass` "/Game/Characters/Boss/Pattern_3.Pattern_3_C" (`KismetMathLibrary.MakeTransform` (`KismetMathLibrary.MakeVector` (.x (`self.K2_GetActorLocation`)) (.y (`self.K2_GetActorLocation`)) -140.0)) "Undefined" "MultiplyWithRoot" null null))
  (set `self.SpawnedPattern` _returnvalue)
  (`KismetSystemLibrary.K2_SetTimerDelegate` (`|CreateDelegate` :!event `RemovePatternEvent`) 2.0))

(fn `Pattern_Attack_04`
  (bind (_returnvalue_x _returnvalue_y) (`KismetMathLibrary.BreakVector` (`self.K2_GetActorLocation`)))
  (bind (_returnvalue_x_2 _returnvalue_y_2) (`KismetMathLibrary.BreakVector` (`self.K2_GetActorLocation`)))
  (`self.BossPlayerTargeting`)
  (`KismetSystemLibrary.PrintString` "Pattern 4")
  (`StateTreeComponent.SendStateTreeEvent` (`self.StateTree`) (make `StateTreeEvent` (struct :`TagName` "Boss.StartPattern")))
  ; Actor 소환 로직
  (`self.PlayAnimMontage` "/Game/Characters/Boss/BossGreat_Sword_Power_Up_Montage.BossGreat_Sword_Power_Up_Montage")
  (bind _returnvalue (`|SpawnActorFromClass` "/Game/Characters/Boss/Pattern_4.Pattern_4_C" (`KismetMathLibrary.MakeTransform` (`KismetMathLibrary.MakeVector` _returnvalue_x _returnvalue_y -140.0)) "Undefined" "MultiplyWithRoot" null null)) ; 패턴 소환
  (bind _returnvalue_2 (`|SpawnActorFromClass` "/Game/Characters/Boss/Pattern_4_Sword.Pattern_4_Sword_C" (`KismetMathLibrary.MakeTransform` (`KismetMathLibrary.MakeVector` _returnvalue_x_2 _returnvalue_y_2 50.0)) "Undefined" "MultiplyWithRoot" null null)) ; 검 이펙트 소환
  (set `self.SpawnedPattern2` _returnvalue)
  ; Actor 사라지는 로직
  (set `self.SpawnSword` _returnvalue_2)
  (`KismetSystemLibrary.K2_SetTimerDelegate` (`|CreateDelegate` :!event `RemoveSword`) 1.5)
  (`KismetSystemLibrary.K2_SetTimerDelegate` (`|CreateDelegate` :!event `RemovePatternEvent2`) 1.0))

(fn `Pattern_Counter`
  (`self.BossPlayerTargeting`)
  (`StateTreeComponent.SendStateTreeEvent` (`self.StateTree`) (make `StateTreeEvent` (struct :`TagName` "Boss.StartCounter"))))

(fn `UpdateBossHP`
  (params (Damage :type "Float (double-precision)"))
  (returns (Bs_Die :type Boolean) (Boss_HP :type "Float (double-precision)"))
  (if (> (`self.Boss_CHP`) 0.0)
    (bind _output_get (set `self.Boss_CHP` (`KismetMathLibrary.FClamp` (- (`self.Boss_CHP`) Damage) 0.0 (`self.Boss_MHP`))))
    (return (<= _output_get 0.0) 0.0)))

(fn `UserConstructionScript`)