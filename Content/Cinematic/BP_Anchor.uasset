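; BP_Anchor is a cinematic anchor actor that spins on yaw, apparently to drive a camera move.
; While IsRotate is set, Tick adds Speed as local yaw each frame, without delta-time scaling.
; CountRotate increments when world yaw lands within a tight tolerance of zero.
; Once the count reaches one, it sets MovingFinish, fires OnCameraFinish and disables its tick.
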(event `self.ReceiveTick`
  (params (DeltaSeconds :type "Float (single-precision)"))
  (bind (_returnvalue_roll _returnvalue_pitch _returnvalue_yaw) (`KismetMathLibrary.BreakRotator` (`self.K2_GetActorRotation`)))
  (if (`self.IsRotate`)
    (if (< (`self.CountRotate`) 1)
      (`self.K2_AddActorLocalRotation` (`KismetMathLibrary.MakeRotator` 0.0 0.0 (`self.Speed`)))
      (if (`KismetMathLibrary.NearlyEqual_FloatFloat` _returnvalue_yaw 0.0 0.001)
        (set `self.CountRotate` (+ (`self.CountRotate`) 1)))
      (else
        (set `self.MovingFinish` true)
        (`self.OnCameraFinish`)
        (`self.SetActorTickEnabled` false)))))

(fn `UserConstructionScript`)