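; Cinematic quick-time-event actor that runs a power clash QTE and reports its result.
; When BP_Anchor cameras finish, it spawns a Niagara clash at the anchors' average location, then after a delay starts camera shake and the W_QTE widget.
; Tick watches IsTimerActive; once false, it saves IsQteResult to BP_GameInstance, tears down the presentation and fires OnQteFinish.
; The countdown and result are not updated in this Blueprint.
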(event `self.ReceiveBeginPlay`
  (set `self.IsTimerActive` true)
  (set `self.CurrentTime` (`self.EndTime`))
  (bind _outactors (`GameplayStatics.GetAllActorsOfClass` "/Game/Cinematic/BP_Anchor.BP_Anchor_C"))
  (add `/Game/Cinematic/BP_Anchor.OnCameraFinish` _outactors (delegate `Start QTE Event`)))

(event `Start QTE Event`
  ; create qte start
  (`self.Effect_start`)
  (`KismetSystemLibrary.Delay` 1.3)
  (`self.CameraMove_start`)
  (`self.UI_start`))

(event `self.ReceiveTick`
  (params (DeltaSeconds :type "Float (single-precision)"))
  (if (not (`self.IsTimerActive`))
    (`self.SetActorTickEnabled` false)
    (bind _asbp_game_instance (cast `/Game/Core/BP_GameInstance` (`GameplayStatics.GetGameInstance`)))
    (set `/Game/Core/BP_GameInstance.KD_Result` (`self.IsQteResult`) _asbp_game_instance)
    ; stop qte event
    (`self.CameraMove_stop`)
    (`self.UI_stop`)
    (`KismetSystemLibrary.Delay` 1.0)
    (`self.Effect_stop`)
    (`self.OnQteFinish`)
    (if (`self.IsQteResult`)
      (`KismetSystemLibrary.PrintText` "Success")
      (else
        (`KismetSystemLibrary.PrintText` "Fail")))))

(fn `CameraMove_start`
  (bind _returnvalue (`PlayerCameraManager.StartCameraShake` :`self` (`GameplayStatics.GetPlayerCameraManager` 0) :`ShakeClass` "/Game/Cinematic/CS_powerstruggle.CS_powerstruggle_C"))
  (set `self.Shake Camera` _returnvalue))

(fn `CameraMove_stop`
  (`PlayerCameraManager.StopCameraShake` (`GameplayStatics.GetPlayerCameraManager` 0) (`self.Shake Camera`) true))

(fn `Effect_start`
  (bind _outactors (`GameplayStatics.GetAllActorsOfClass` "/Game/Cinematic/BP_Anchor.BP_Anchor_C"))
  (bind _returnvalue (`GameplayStatics.GetActorArrayAverageLocation` _outactors))
  (bind _returnvalue_2 (`NiagaraFunctionLibrary.SpawnSystemAtLocation` "/Game/Cinematic/NS_PowerClash.NS_PowerClash" _returnvalue))
  (set `self.Effect` _returnvalue_2))

(fn `Effect_stop`
  (`ActorComponent.Deactivate` (`self.Effect`)))

(fn `UI_start`
  (bind _returnvalue (`|CreateWidget` "/Game/Cinematic/W_QTE.W_QTE_C" (`GameplayStatics.GetPlayerController` 0)))
  (bind _output_get (set `self.Widget` _returnvalue))
  (`UserWidget.AddToViewport` _output_get 0))

(fn `UI_stop`
  (`Widget.RemoveFromParent` (`self.Widget`)))

(fn `UserConstructionScript`)