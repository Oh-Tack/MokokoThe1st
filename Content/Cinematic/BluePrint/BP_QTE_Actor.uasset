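; Cinematic actor that runs a power-clash quick-time event (QTE) once the BP_Anchor actors signal camera finish.
; Start spawns a Niagara clash effect at the anchors' average location, then after a delay adds camera shake and two QTE widgets.
; Tick waits for IsTimerActive to clear, writes the result to BP_PlayerState.ClashResult, tears everything down and calls OnQteFinish.
; The countdown and result are not updated in this graph.
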(event `self.ReceiveBeginPlay`
  (set `self.IsTimerActive` true)
  (set `self.CurrentTime` (`self.EndTime`))
  (bind _outactors (`GameplayStatics.GetAllActorsOfClass` "/Game/Cinematic/BP_Anchor.BP_Anchor_C"))
  (add `/Game/Cinematic/BP_Anchor.OnCameraFinish` _outactors (delegate `Start QTE Event`)))

(event `Start QTE Event`
  ; create qte start
  (`self.Effect_start`)
  (`KismetSystemLibrary.Delay` 1.3)
  (`self.CameraMove_start`)
  (`self.UI_start`))

(event `self.ReceiveTick`
  (params (DeltaSeconds :type "Float (single-precision)"))
  (if (not (`self.IsTimerActive`))
    (`self.SetActorTickEnabled` false)
    (bind _returnvalue (`GameplayStatics.GetActorOfClass` "/Game/Cinematic/BluePrint/BP_PlayerState.BP_PlayerState_C"))
    (set `/Game/Cinematic/BluePrint/BP_PlayerState.Clash_Result` (`self.IsQteResult`) _returnvalue)
    ; stop qte event
    (`self.CameraMove_stop`)
    (`self.UI_stop`)
    (`KismetSystemLibrary.Delay` 1.0)
    (`self.Effect_stop`)
    (`self.OnQteFinish`)
    (if (`self.IsQteResult`)
      (`KismetSystemLibrary.PrintText` "Success")
      (else
        (`KismetSystemLibrary.PrintText` "Fail" :!label _label)))))

(event `Key|One`
  (params (Key :type "Key Structure"))
  (:`Pressed`
    (goto _label)))

(fn `CameraMove_start`
  (bind _returnvalue (`PlayerCameraManager.StartCameraShake` :`self` (`GameplayStatics.GetPlayerCameraManager` 0) :`ShakeClass` "/Game/Cinematic/BluePrint/Camera/CS_ClashShake.CS_ClashShake_C"))
  (set `self.Shake Camera` _returnvalue))

(fn `CameraMove_stop`
  (`PlayerCameraManager.StopCameraShake` (`GameplayStatics.GetPlayerCameraManager` 0) (`self.Shake Camera`) true))

(fn `Effect_start`
  (bind _outactors (`GameplayStatics.GetAllActorsOfClass` "/Game/Cinematic/BP_Anchor.BP_Anchor_C"))
  (bind _returnvalue (`GameplayStatics.GetActorArrayAverageLocation` _outactors))
  (bind _returnvalue_2 (`NiagaraFunctionLibrary.SpawnSystemAtLocation` "/Game/Cinematic/Particle/NS_PowerClash.NS_PowerClash" _returnvalue))
  (set `self.Effect` _returnvalue_2))

(fn `Effect_stop`
  (`ActorComponent.Deactivate` (`self.Effect`)))

(fn `UI_start`
  (bind _returnvalue (`|CreateWidget` "/Game/Cinematic/BluePrint/W_QTE.W_QTE_C" (`GameplayStatics.GetPlayerController` 0)))
  (bind _output_get (set `self.Widget` _returnvalue))
  (`UserWidget.AddToViewport` _output_get 0)
  (bind _returnvalue_2 (`|CreateWidget` "/Game/Cinematic/BluePrint/WBP_Qte.WBP_Qte_C" (`GameplayStatics.GetPlayerController` 0)))
  (bind _output_get_2 (set `self.PartUI` _returnvalue_2))
  (`UserWidget.AddToViewport` _output_get_2 0))

(fn `UI_stop`
  (`Widget.RemoveFromParent` (`self.Widget`))
  (`Widget.RemoveFromParent` (`self.PartUI`)))

(fn `UserConstructionScript`)