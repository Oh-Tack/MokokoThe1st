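; BP_EnterClash is an actor in the Cinematic folder that shows a widget while something is inside its Collision_Range volume.
; BeginPlay hides the widget, then begin and end overlap on Collision_Range set the WidgetVisibility flag and apply it to the widget.
; The overlap handlers do not filter which actor triggers them, and visibility changes are not propagated to child components.
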(event `self.ReceiveBeginPlay`
  (set `self.Widget_Visibility` false)
  (`SceneComponent.SetVisibility` (`self.Widget`) (`self.Widget_Visibility`) false))

(event `self.Collision_Range.OnComponentBeginOverlap`
  (params (OverlappedComponent :type "PrimitiveComponent Object Reference") (OtherActor :type "Actor Object Reference") (OtherComp :type "PrimitiveComponent Object Reference") (OtherBodyIndex :type Integer) (bFromSweep :type Boolean) (SweepResult :type "HitResult Structure (by ref)"))
  (set `self.Widget_Visibility` true)
  (`SceneComponent.SetVisibility` (`self.Widget`) (`self.Widget_Visibility`) false))

(event `self.Collision_Range.OnComponentEndOverlap`
  (params (OverlappedComponent :type "PrimitiveComponent Object Reference") (OtherActor :type "Actor Object Reference") (OtherComp :type "PrimitiveComponent Object Reference") (OtherBodyIndex :type Integer))
  (set `self.Widget_Visibility` false)
  (`SceneComponent.SetVisibility` (`self.Widget`) (`self.Widget_Visibility`) false))

(fn `UserConstructionScript`)