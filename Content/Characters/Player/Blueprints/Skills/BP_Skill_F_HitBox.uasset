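; BP_Skill_F_HitBox is the hitbox actor for the player's F skill, dealing heavy fixed damage to the boss.
; On BeginPlay it caches a single BP_Enemy found by class as the boss, plus the player character and controller, which are otherwise unused here.
; When an overlapping actor matches that boss, it applies damage tagged with the BP_Player_Skill_F damage type, ignoring all other actors.
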(event `self.ReceiveBeginPlay`
  (bind _returnvalue (`GameplayStatics.GetActorOfClass` "/Game/Blueprints/Boss/BP_Enemy.BP_Enemy_C"))
  (set `self.Boss` _returnvalue)
  (bind _asbp_player_charater (cast `/Game/Characters/Player/Blueprints/BP_PlayerCharater` (`GameplayStatics.GetPlayerCharacter` 0)))
  (set `self.As BP Player Charater` _asbp_player_charater)
  (bind _asbp_player_controller (cast `/Game/Characters/Player/Blueprints/BP_PlayerController` (`GameplayStatics.GetPlayerController` 0)))
  (set `self.As BP Player Controller` _asbp_player_controller))

(event `self.ReceiveActorBeginOverlap`
  (params (OtherActor :type "Actor Object Reference"))
  (bind _boss (`self.Boss`))
  (if (== OtherActor _boss)
    (`GameplayStatics.ApplyDamage` _boss 30000.0 null null "/Game/Core/BP_Player_Skill_F.BP_Player_Skill_F_C")))

(fn `UserConstructionScript`)