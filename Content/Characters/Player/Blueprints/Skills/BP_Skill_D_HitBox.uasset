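; Hitbox actor for the player's hold-and-release Skill D, damaging the single boss found at BeginPlay.
; Overlapping the boss sets a Hit flag, letting Tick deal periodic damage while the player controller reports holding.
; Releasing after a hit deals one finishing blow, doubled on a perfect release; full holding power triggers the base finisher without checking Hit.
; Overlap and finish events switch collision responses on the tick and finish shapes.
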(event `self.ReceiveBeginPlay`
  (bind _returnvalue (`GameplayStatics.GetActorOfClass` "/Game/Blueprints/Boss/BP_Enemy.BP_Enemy_C"))
  (set `self.Boss` _returnvalue)
  (bind _asbp_player_charater (cast `/Game/Characters/Player/Blueprints/BP_PlayerCharater` (`GameplayStatics.GetPlayerCharacter` 0)))
  (set `self.As BP Player Charater` _asbp_player_charater)
  (bind _asbp_player_controller (cast `/Game/Characters/Player/Blueprints/BP_PlayerController` (`GameplayStatics.GetPlayerController` 0)))
  (set `self.As BP Player Controller` _asbp_player_controller))

(event `self.ReceiveTick`
  (params (DeltaSeconds :type "Float (single-precision)"))
  (if (< (`/Game/Characters/Player/Blueprints/BP_PlayerController.Skill_D_Holding_Power` (`self.As BP Player Controller`)) 1.0)
    (`|ExecutionSequence`
      (:`then_0`
        (if (and (`/Game/Characters/Player/Blueprints/BP_PlayerController.bSkill_D_Holding` (`self.As BP Player Controller`)) (`self.bHit`))
          (bind _output_get (set `self.currTime` (+ DeltaSeconds (`self.currTime`))))
          (if (> _output_get (`self.tickTime`))
            (`GameplayStatics.ApplyDamage` (`self.Boss`) 1000.0 null null "/Game/Core/BP_Player_Skill_D.BP_Player_Skill_D_C")
            (set `self.currTime` 0.0))))
      (:`then_1`
        (if (and (not (`/Game/Characters/Player/Blueprints/BP_PlayerController.bSkill_D_Holding` (`self.As BP Player Controller`))) (`self.bHit`))
          (`/Engine/EditorBlueprintResources/StandardMacros.DoOnce` false
            (:`Completed`
              (`PrimitiveComponent.SetCollisionResponseToChannel` (`self.Skill_D_Finish`) "ECC_GameTraceChannel4" "ECR_Overlap")
              (if (`/Game/Characters/Player/Blueprints/BP_PlayerController.bSkill_D_Perfect` (`self.As BP Player Controller`))
                (set `self.Skill_D_Damage` 20000.0)
                (else
                  (set `self.Skill_D_Damage` 10000.0)))
              (`GameplayStatics.ApplyDamage` (`self.Boss`) (`self.Skill_D_Damage`) null null "/Game/Core/BP_Player_Skill_D.BP_Player_Skill_D_C"))))))
    (else
      (`/Engine/EditorBlueprintResources/StandardMacros.DoOnce` false
        (:`Completed`
          (`PrimitiveComponent.SetCollisionResponseToChannel` (`self.Skill_D_Finish`) "ECC_GameTraceChannel4" "ECR_Overlap")
          (bind _output_get_2 (set `self.Skill_D_Damage` 10000.0))
          (`GameplayStatics.ApplyDamage` (`self.Boss`) _output_get_2 null null "/Game/Core/BP_Player_Skill_D.BP_Player_Skill_D_C"))))))

(event `self.ReceiveActorBeginOverlap`
  (params (OtherActor :type "Actor Object Reference"))
  (`PrimitiveComponent.SetCollisionResponseToChannel` (`self.Skill_D_Finish`) "ECC_GameTraceChannel4" "ECR_Ignore")
  (`PrimitiveComponent.SetCollisionResponseToChannel` (`self.Skill_D_Tick`) "ECC_GameTraceChannel4" "ECR_Overlap")
  (if (== OtherActor (`self.Boss`))
    (set `self.currTime` 0.0)
    (set `self.bHit` true)))

(fn `UserConstructionScript`)