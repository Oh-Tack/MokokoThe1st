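; BP_Dummy is a test dummy for the player's counter mechanic against an enemy counter state.
; Tick feeds a five-second Delay into a FlipFlop that toggles the CounterSkill flag on and off.
; When DummyCollision is overlapped while the flag is set, it compares the other component to the cached player's PlayerAttackRange and, on a match, prints a counter message.
; Detection only produces debug prints, with no further gameplay response.
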(event `self.ReceiveBeginPlay`
  (`KismetSystemLibrary.PrintString` (`KismetStringLibrary.Conv_BoolToString` (`self.bCounterSkill`)))
  (bind _asbp_player_charater (cast `/Game/Characters/Player/Blueprints/BP_PlayerCharater` (`GameplayStatics.GetPlayerCharacter` 0)))
  (set `self.As BP Player Charater` _asbp_player_charater))

(event `self.ReceiveTick`
  (params (DeltaSeconds :type "Float (single-precision)"))
  ; 5초 마다 더미가 카운터 스킬을 5초 동안 발동함
  (`KismetSystemLibrary.Delay` 5.0)
  (`/Engine/EditorBlueprintResources/StandardMacros.FlipFlop`
    (:`A`
      (bind _output_get (set `self.bCounterSkill` true))
      (`KismetSystemLibrary.PrintString` (`KismetStringLibrary.Conv_BoolToString` _output_get)))
    (:`B`
      (bind _output_get_2 (set `self.bCounterSkill` false))
      (`KismetSystemLibrary.PrintString` (`KismetStringLibrary.Conv_BoolToString` _output_get_2)))))

(event `self.DummyCollision.OnComponentBeginOverlap`
  (params (OverlappedComponent :type "PrimitiveComponent Object Reference") (OtherActor :type "Actor Object Reference") (OtherComp :type "PrimitiveComponent Object Reference") (OtherBodyIndex :type Integer) (bFromSweep :type Boolean) (SweepResult :type "HitResult Structure (by ref)"))
  (`KismetSystemLibrary.PrintString` (`KismetSystemLibrary.GetDisplayName` OtherComp))
  (if (and (`self.bCounterSkill`) (== OtherComp (`/Game/Characters/Player/Blueprints/BP_PlayerCharater.PlayerAttackRange` (`self.As BP Player Charater`))))
    (`KismetSystemLibrary.PrintString` "Counter!!!!!!")))

(fn `UserConstructionScript`)