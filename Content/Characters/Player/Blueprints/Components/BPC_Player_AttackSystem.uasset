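; Player attack component that runs a three-hit melee-style montage combo on left mouse input for BP_PlayerCharater.
; An attack needs CanAttack, no attack in progress and a specific skill enum; it halts movement and sets the player state.
; Montage notifies clear IsAttacking and advance or wrap ComboCounter, opening the next hit.
; A timer event, ResetCounter, zeroes the combo and restores the default state unless another state blocks it.
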(event `self.ReceiveBeginPlay`
  (bind _asbp_player_charater (cast `/Game/Characters/Player/Blueprints/BP_PlayerCharater` (`self.GetOwner`)))
  (bind _output_get (set `self.As BP Player Charater` _asbp_player_charater))
  (set `self.PlayerMesh` (`Character.Mesh` _output_get)))

(event `EnhancedInput|/Game/Inputs/Actions/IA_Mouse_Left`
  (params (ActionValue :type Boolean) (ElapsedSeconds :type "Float (double-precision)") (TriggeredSeconds :type "Float (double-precision)") (InputAction :type "InputAction Object Reference" :default "/Game/Inputs/Actions/IA_Mouse_Left.IA_Mouse_Left"))
  (bind _as_bp_player_charater (`self.As BP Player Charater`))
  (bind _playermesh (`self.PlayerMesh`))
  ; 콤보 공격 로직
  (:`Triggered`
    (if (and (not (`self.bIsAttacking`)) (`self.bCanAttack`) (`|EnumEquality` (`/Game/Characters/Player/Blueprints/BP_PlayerCharater.EPlayerSkill` (`self.As BP Player Charater`)) "NewEnumerator2")) :!label _label
      (`MovementComponent.StopMovementImmediately` (`Character.CharacterMovement` (`self.As BP Player Charater`)))
      (set `/Game/Characters/Player/Blueprints/BP_PlayerCharater.EPlayerState` "NewEnumerator2" _as_bp_player_charater)
      (set `/Game/Characters/Player/Blueprints/BP_PlayerCharater.EPlayerSkill` "NewEnumerator2" _as_bp_player_charater)
      (set `self.bIsAttacking` true)
      (switch `int` (`self.ComboCounter`)
        (:`0`
          (`|PlayMontage` _playermesh "/Game/Characters/Player/Animations/Attack/Player_ComboAttack1_Montage.Player_ComboAttack1_Montage" 1.0 0.0 "None" false
            (:`then`
              (`KismetSystemLibrary.K2_SetTimerDelegate` (delegate `ResetCounter`) 1.0 :!label _label_2))
            (:`OnNotifyBegin`
              (set `self.bIsAttacking` false)
              (set `self.ComboCounter` 1))))
        (:`1`
          (`|PlayMontage` _playermesh "/Game/Characters/Player/Animations/Attack/Player_ComboAttack2_Montage.Player_ComboAttack2_Montage" 0.5
            (:`then`
              (goto _label_2))
            (:`OnNotifyBegin`
              (set `self.bIsAttacking` false)
              (set `self.ComboCounter` 2))))
        (:`2`
          (`|PlayMontage` _playermesh "/Game/Characters/Player/Animations/Attack/Player_ComboAttack3_Montage.Player_ComboAttack3_Montage"
            (:`then`
              (`KismetSystemLibrary.K2_SetTimerDelegate` (delegate `ResetCounter`) 1.85))
            (:`OnNotifyBegin`
              (set `self.bIsAttacking` false)
              (set `self.ComboCounter` 0)))))))
  (:`Started`
    (goto _label)))

(event `ResetCounter`
  ; 콤보 공격 로직
  (set `self.ComboCounter` 0)
  (if (not (`|EnumEquality` (`/Game/Characters/Player/Blueprints/BP_PlayerCharater.EPlayerState` (`self.As BP Player Charater`)) "NewEnumerator1"))
    (set `/Game/Characters/Player/Blueprints/BP_PlayerCharater.EPlayerState` "NewEnumerator0" (`self.As BP Player Charater`))))