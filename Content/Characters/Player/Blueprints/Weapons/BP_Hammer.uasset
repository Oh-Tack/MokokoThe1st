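; BP_Hammer is the player's hammer weapon, damaging the boss when its attack collision begins overlapping it.
; Shortly after BeginPlay it caches the first BP_Enemy found as the boss, along with a reference to the player character.
; On a boss overlap, the player's current skill selects normal-attack or heavier Skill A damage, each with its own damage type, then a Niagara hit effect spawns at the boss's location.
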(event `self.ReceiveBeginPlay`
  (`KismetSystemLibrary.Delay` 0.5)
  (bind _returnvalue (`GameplayStatics.GetActorOfClass` "/Game/Blueprints/Boss/BP_Enemy.BP_Enemy_C"))
  (set `self.Boss` _returnvalue)
  (bind _asbp_player_charater (cast `/Game/Characters/Player/Blueprints/BP_PlayerCharater` (`GameplayStatics.GetPlayerCharacter` 0)))
  (set `self.As BP Player Charater` _asbp_player_charater))

(event `self.ReceiveTick`
  (params (DeltaSeconds :type "Float (single-precision)")))

(event `self.HammerAttackCollision.OnComponentBeginOverlap`
  (params (OverlappedComponent :type "PrimitiveComponent Object Reference") (OtherActor :type "Actor Object Reference") (OtherComp :type "PrimitiveComponent Object Reference") (OtherBodyIndex :type Integer) (bFromSweep :type Boolean) (SweepResult :type "HitResult Structure (by ref)"))
  (bind _boss (`self.Boss`))
  (`KismetSystemLibrary.PrintString` "Hello")
  (if (== OtherActor _boss)
    (`|ExecutionSequence`
      (:`then_0`
        (switch `/Game/Core/E_PlayerAttackType` (`/Game/Characters/Player/Blueprints/BP_PlayerCharater.EPlayerSkill` (`self.As BP Player Charater`))
          (:`NewEnumerator2`
            (`GameplayStatics.ApplyDamage` _boss 1000.0 null null "/Game/Core/BP_Player_NormalAttack.BP_Player_NormalAttack_C"))
          (:`NewEnumerator0`
            (`GameplayStatics.ApplyDamage` _boss 2000.0 null null "/Game/Core/BP_Player_Skill_A.BP_Player_Skill_A_C"))))
      (:`then_1`
        (`NiagaraFunctionLibrary.SpawnSystemAtLocation` "/Game/Effects/PlayerSkill/NS_HitEffect.NS_HitEffect" (`self.K2_GetActorLocation` (`self.Boss`)) (struct) (2.0 2.0 2.0))))))

(fn `UserConstructionScript`)