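; BP_Weapon_Collision is an anim notify state that opens a melee hit window on the player character during attack animations.
; On begin, it casts the mesh owner to BP_PlayerCharater and sets its PlayerAttackRange collision response on GameTraceChannel4 to Overlap.
; On end, it sets that response back to Ignore, and both events print debug strings.
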(fn `Received_NotifyBegin`
  (params (MeshComp :type "SkeletalMeshComponent Object Reference") (Animation :type "AnimSequenceBase Object Reference") (TotalDuration :type "Float (single-precision)") (EventReference :type "AnimNotifyEventReference Structure (by ref)"))
  (returns (ReturnValue :type Boolean))
  (bind _asbp_player_charater (cast `/Game/Characters/Player/Blueprints/BP_PlayerCharater` (`ActorComponent.GetOwner` MeshComp)))
  (`PrimitiveComponent.SetCollisionResponseToChannel` (`/Game/Characters/Player/Blueprints/BP_PlayerCharater.PlayerAttackRange` _asbp_player_charater) "ECC_GameTraceChannel4" "ECR_Overlap")
  (`KismetSystemLibrary.PrintString` null "Begin")
  (return false))

(fn `Received_NotifyEnd`
  (params (MeshComp :type "SkeletalMeshComponent Object Reference") (Animation :type "AnimSequenceBase Object Reference") (EventReference :type "AnimNotifyEventReference Structure (by ref)"))
  (returns (ReturnValue :type Boolean))
  (bind _asbp_player_charater (cast `/Game/Characters/Player/Blueprints/BP_PlayerCharater` (`ActorComponent.GetOwner` MeshComp)))
  (`PrimitiveComponent.SetCollisionResponseToChannel` (`/Game/Characters/Player/Blueprints/BP_PlayerCharater.PlayerAttackRange` _asbp_player_charater) "ECC_GameTraceChannel4" "ECR_Ignore")
  (`KismetSystemLibrary.PrintString` null "End")
  (return false))