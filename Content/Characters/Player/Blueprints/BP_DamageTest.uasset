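; BP_DamageTest is an actor for testing light and heavy damage on whatever overlaps it.
; On BeginPlay its TextRender displays the selected DamageType as a label.
; On overlap it switches on DamageType, applies a smaller or much larger damage amount with the matching damage type class, and prints which kind fired.
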(event `self.ReceiveBeginPlay`
  (`TextRenderComponent.K2_SetText` (`self.TextRender`) (`KismetTextLibrary.Conv_StringToText` (`self.DamageType`))))

(event `self.ReceiveActorBeginOverlap`
  (params (OtherActor :type "Actor Object Reference"))
  (switch `string` (`self.DamageType`)
    (:`Light`
      (`GameplayStatics.ApplyDamage` OtherActor 50.0 null null "/Game/Core/BP_DamageType_Light.BP_DamageType_Light_C")
      (`KismetSystemLibrary.PrintString` "Light"))
    (:`Heavy`
      (`GameplayStatics.ApplyDamage` OtherActor 1000.0 null null "/Game/Core/BP_DamageType_heavy.BP_DamageType_heavy_C")
      (`KismetSystemLibrary.PrintString` "Heavy"))))

(fn `UserConstructionScript`)