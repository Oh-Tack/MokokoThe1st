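; Player controller for click-to-move control and skill input, driving BP_PlayerCharater through Enhanced Input and raw key events.
; Holding right mouse steers the pawn toward the cursor, while a short click uses SimpleMoveToLocation with a cursor effect.
; D and F show hold/charge widgets as Tick builds their power, firing on release or at full charge.
; Tick also caches the cursor hit location, and releasing S casts only if in range.
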(event `self.ReceiveTick`
  (params (DeltaSeconds :type "Float (single-precision)"))
  (`|ExecutionSequence`
    (:`then_0`
      (set `self.CursorUnderHit` (`.Location` (`GameplayStatics.BreakHitResult` (`self.GetHitResultUnderCursorByChannel` (`GameplayStatics.GetPlayerController` 0) "TraceTypeQuery1" true)))))
    (:`then_1`
      ; Skill D
      (if (not (not (`self.bSkill_D_Holding`)))
        (bind _output_get (set `self.Skill_D_Holding_Curr_Time` (+ DeltaSeconds (`self.Skill_D_Holding_Curr_Time`))))
        (bind _output_get_2 (set `self.Skill_D_Holding_Power` (`KismetMathLibrary.FClamp` (/ _output_get (`self.Skill_D_Holding_Max_Time`)))))
        (`KismetSystemLibrary.PrintString` (`KismetStringLibrary.Conv_DoubleToString` _output_get_2))
        (if (>= _output_get_2 1.0)
          (set `self.bSkill_D_Holding` false)
          (`/Game/Characters/Player/Blueprints/BP_PlayerCharater.Skill_D` (`self.As BP Player Charater`))
          (`KismetSystemLibrary.Delay` 0.3)
          (`Widget.RemoveFromParent` (`self.Skill_D_HoldBar`)))))
    (:`then_2`
      (if (not (not (`self.bSkill_F_Holding`)))
        (bind _output_get_3 (set `self.Skill_F_Holding_Curr_Time` (+ DeltaSeconds (`self.Skill_F_Holding_Curr_Time`))))
        (bind _output_get_4 (set `self.Skill_F_Holding_Power` (`KismetMathLibrary.FClamp` (/ _output_get_3 (`self.Skill_F_Holding_Max_Time`)))))
        (`KismetSystemLibrary.PrintString` (`KismetStringLibrary.Conv_DoubleToString` _output_get_4))
        (if (>= _output_get_4 1.0)
          (set `self.bSkill_F_Holding` false)
          (`/Game/Characters/Player/Blueprints/BP_PlayerCharater.Skill_F` (`self.As BP Player Charater`))
          (`KismetSystemLibrary.Delay` 0.3)
          (`Widget.RemoveFromParent` (`self.Skill_F_Charge_bar`)))))))

(event `Key|D`
  (params (Key :type "Key Structure"))
  (bind _as_bp_player_charater (`self.As BP Player Charater`))
  ; Skill D
  (:`Pressed`
    (if (`/Game/Characters/Player/Blueprints/BP_PlayerCharater.bCanSkill_D` _as_bp_player_charater)
      (`/Game/Characters/Player/Blueprints/BP_PlayerCharater.Time_Remaining_Skill_D` _as_bp_player_charater)
      (set `self.bSkill_D_Holding` true)
      (set `self.Skill_D_Holding_Curr_Time` 0.0)
      (set `self.Skill_D_Holding_Power` 0.0)
      (bind _returnvalue (`|CreateWidget` "/Game/UI/Widgets/WB_HoldingBar.WB_HoldingBar_C" self))
      (bind _output_get (set `self.Skill_D_HoldBar` _returnvalue))
      (`UserWidget.AddToViewport` _output_get 1)))
  (:`Released`
    (set `self.bSkill_D_Holding` false)
    (if (< (`self.Skill_D_Holding_Power`) 1.0)
      (`/Game/Characters/Player/Blueprints/BP_PlayerCharater.Skill_D` _as_bp_player_charater)
      (`KismetSystemLibrary.Delay` 0.3)
      (`Widget.RemoveFromParent` (`self.Skill_D_HoldBar`)))))

(event `self.ReceiveBeginPlay`
  (bind _returnvalue (subsystem `EnhancedInputLocalPlayerSubsystem`))
  ; Enhanced Input 및 초기 설정
  (`/Engine/EditorBlueprintResources/StandardMacros.IsValid` _returnvalue
    (:`Is Valid`
      (`EnhancedInputSubsystemInterface.AddMappingContext` _returnvalue "/Game/Inputs/IMC_PlayerInput.IMC_PlayerInput" 0 (struct))
      (bind _asbp_player_charater (cast `/Game/Characters/Player/Blueprints/BP_PlayerCharater` (`GameplayStatics.GetPlayerCharacter` 0)))
      (set `self.As BP Player Charater` _asbp_player_charater))))

(event `Key|F`
  (params (Key :type "Key Structure"))
  (bind _as_bp_player_charater (`self.As BP Player Charater`))
  (:`Pressed`
    (if (`/Game/Characters/Player/Blueprints/BP_PlayerCharater.bCanSkill_F` _as_bp_player_charater)
      (`/Game/Characters/Player/Blueprints/BP_PlayerCharater.Time_Remaining_Skill_F` _as_bp_player_charater)
      (set `self.bSkill_F_Holding` true)
      (set `self.Skill_F_Holding_Curr_Time` 0.0)
      (set `self.Skill_F_Holding_Power` 0.0)
      (bind _returnvalue (`|CreateWidget` "/Game/UI/Widgets/WB_ChargingBar.WB_ChargingBar_C" self))
      (bind _output_get (set `self.Skill_F_Charge_bar` _returnvalue))
      (`UserWidget.AddToViewport` _output_get 1)))
  (:`Released`
    (set `self.bSkill_F_Holding` false)
    (if (< (`self.Skill_F_Holding_Power`) 1.0)
      (`/Game/Characters/Player/Blueprints/BP_PlayerCharater.Skill_F` _as_bp_player_charater)
      (`KismetSystemLibrary.Delay` 0.3)
      (`Widget.RemoveFromParent` (`self.Skill_F_Charge_bar`)))))

(event `EnhancedInput|/Game/Inputs/Actions/IA_Mouse_Right`
  (params (ActionValue :type Boolean) (ElapsedSeconds :type "Float (double-precision)") (TriggeredSeconds :type "Float (double-precision)") (InputAction :type "InputAction Object Reference" :default "/Game/Inputs/Actions/IA_Mouse_Right.IA_Mouse_Right"))
  (bind (_hit _loc) (`self.GetLocationUnderCursor`))
  (bind (_hit_2 _loc_2) (`self.GetLocationUnderCursor`))
  (bind _as_bp_player_charater (`self.As BP Player Charater`))
  (bind _returnvalue (and (`|EnumEquality` (`/Game/Characters/Player/Blueprints/BP_PlayerCharater.EPlayerState` _as_bp_player_charater) "NewEnumerator0") (not (`/Game/Characters/Player/Blueprints/BP_PlayerCharater.bWakeUpActing` _as_bp_player_charater))))
  ; 오른쪽 마우스 클릭 - 이동
  (:`Triggered`
    (if _returnvalue
      (if _hit
        (bind _output_get (set `self.CachedDestination` _loc))
        (`self.Follow` _output_get))))
  (:`Started`
    (`self.StopMovement`)
    (if _hit_2
      (set `self.CachedDestination` _loc_2)))
  (:`Canceled`
    (if _returnvalue :!label _label
      (if (< ElapsedSeconds (`self.PressedThreshold`))
        (`self.MoveTo` (`self.CachedDestination`)))))
  (:`Completed`
    (goto _label)))

(event `Key|S`
  (params (Key :type "Key Structure"))
  (bind _as_bp_player_charater (`self.As BP Player Charater`))
  ; Skill S
  (:`Pressed`
    (set `self.bSkill_S_Hoding` true))
  (:`Released`
    (set `self.bSkill_S_Hoding` false)
    (if (`/Game/Characters/Player/Blueprints/BP_PlayerCharater.bCanSkill_S` _as_bp_player_charater)
      (set `/Game/Characters/Player/Blueprints/BP_PlayerCharater.bCanSkill_S` false _as_bp_player_charater)
      (if (`/Game/Characters/Player/Blueprints/BP_PlayerCharater.bSkill_S_InCircle` _as_bp_player_charater)
        (`/Game/Characters/Player/Blueprints/BP_PlayerCharater.Skill_S` _as_bp_player_charater)
        (`/Game/Characters/Player/Blueprints/BP_PlayerCharater.Time_Remaining_Skill_S` _as_bp_player_charater)
        (else
          (`KismetSystemLibrary.PrintString` "사정거리 벗어남"))))
    (`/Game/Characters/Player/Blueprints/BP_PlayerCharater.DestroyDecalSkill_S` _as_bp_player_charater)))

(fn `Follow`
  (params (Loc :type "Vector Structure"))
  (bind _returnvalue (`self.K2_GetPawn`))
  (`Pawn.AddMovementInput` _returnvalue (`KismetMathLibrary.GetDirectionUnitVector` (`self.K2_GetActorLocation` _returnvalue) Loc) 1.0 false))

(fn `GetLocationUnderCursor`
  (returns (Hit :type Boolean) (Loc :type "Vector Structure"))
  (bind (_bblockinghit _binitialoverlap _time _distance _location) (`GameplayStatics.BreakHitResult` (`self.GetHitResultUnderCursorByChannel` "TraceTypeQuery1")))
  (return _bblockinghit _location))

(fn `MoveTo`
  (params (Loc :type "Vector Structure"))
  (`AIBlueprintHelperLibrary.SimpleMoveToLocation` self Loc)
  (`NiagaraFunctionLibrary.SpawnSystemAtLocation` "/Game/UI/Cursor/FX_Cursor.FX_Cursor" Loc))

(fn `UserConstructionScript`)